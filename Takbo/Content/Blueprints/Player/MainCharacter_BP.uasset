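; MainCharacter_BP is the player character Blueprint, handling stepped 90-degree camera turns and showing the inventory HUD.
; TurnRight and TurnLeft inputs each pass their own DoOnce, set the turn direction, then share one path computing a rounded target yaw.
; The CamRotateLerp timeline interpolates CameraBoom's world yaw, preserving pitch and roll, and resets both DoOnce gates when finished.
; BeginPlay creates the Inventory widget and adds it to the viewport.
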(event `InputAction|TurnRight`
  (params (Key :type "Key Structure"))
  (bind _cameraboom (`self.CameraBoom`))
  (bind (_returnvalue_roll _returnvalue_pitch _returnvalue_yaw) (`KismetMathLibrary.BreakRotator` (`SceneComponent.K2_GetComponentRotation` (`self.CameraBoom`))))
  (bind (_returnvalue_roll_2 _returnvalue_pitch_2) (`KismetMathLibrary.BreakRotator` (`SceneComponent.K2_GetComponentRotation` _cameraboom)))
  (:`Pressed`
    (`/Engine/EditorBlueprintResources/StandardMacros.DoOnce` false :!label _label
      (:`Completed`
        (set `self.RotateDir` 90.0)
        (bind _output_get (set `self.OldCamRot` _returnvalue_yaw :!label _label_2))
        (set `self.NewCamRot` (`KismetMathLibrary.Conv_IntToDouble` (`KismetMathLibrary.Round` (+ _output_get (`self.RotateDir`)))))
        (bind (_direction _lerpvalue) (`Timeline|CamRotateLerp` :!via `PlayFromStart`)
          (:`Update`
            (`SceneComponent.K2_SetWorldRotation` _cameraboom (`KismetMathLibrary.MakeRotator` _returnvalue_roll_2 _returnvalue_pitch_2 (`KismetMathLibrary.Lerp` (`self.OldCamRot`) (`self.NewCamRot`) _lerpvalue)) false false))
          (:`Finished`
            (`|ExecutionSequence`
              (:`then_0`
                (goto _label :!via `Reset`))
              (:`then_1`
                (goto _label_3 :!via `Reset`)))))))))

(event `InputAction|TurnLeft`
  (params (Key :type "Key Structure"))
  (:`Pressed`
    (`/Engine/EditorBlueprintResources/StandardMacros.DoOnce` false :!label _label_3
      (:`Completed`
        (set `self.RotateDir` -90.0)
        (goto _label_2)))))

(event `self.ReceiveBeginPlay`
  ;[1 1 1] Shows Inventory HUD
  (bind _returnvalue (`|CreateWidget` "/Game/UI/Inventory.Inventory_C" (`GameplayStatics.GetPlayerController` 0)))
  (`UserWidget.AddToViewport` _returnvalue 0))

(fn `UserConstructionScript`)